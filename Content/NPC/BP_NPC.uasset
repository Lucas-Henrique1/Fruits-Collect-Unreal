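; BP_NPC is an AI character that wanders the map and chases pawns it sees.
; Roaming walks slowly to a random reachable point within a radius, pauses briefly at random, then repeats after each successful move.
; PawnSensing sightings raise walk speed and move it toward the seen pawn, while a retriggerable delay returns it to roaming once sightings stop for a few seconds.
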(event `self.ReceiveBeginPlay`
  ;[1 1 1] Start
  (`self.Roaming`))

(event `Roaming`
  ;[1 1 1] Andar pelo mapa
  (set `CharacterMovementComponent.MaxWalkSpeed` 150.0 (`self.CharacterMovement`))
  (`|AIMoveTo` self (`NavigationSystemV1.K2_GetRandomReachablePointInRadius` (`SceneComponent.K2_GetComponentLocation` (`self.Mesh`)) 1000.0 null null) null
    (:`OnSuccess`
      (`KismetSystemLibrary.Delay` (`KismetMathLibrary.RandomFloatInRange` 1.0 4.0))
      (`self.Roaming`))))

(event `self.PawnSensing.OnSeePawn`
  (params (Pawn :type "Pawn Object Reference"))
  ;[1 1 1] Segue o player
  (set `CharacterMovementComponent.MaxWalkSpeed` 300.0 (`self.CharacterMovement`))
  (`|ExecutionSequence`
    (:`then_0`
      (`|AIMoveTo` self (0.0 0.0 0.0) Pawn))
    (:`then_1`
      (`KismetSystemLibrary.RetriggerableDelay` 3.0)
      (`self.Roaming`))))

(fn `UserConstructionScript`)